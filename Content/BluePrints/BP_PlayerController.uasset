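; BP_PlayerController is a player controller that sets up the in-game HUD for the player.
; On BeginPlay it creates a GameHud widget, adds it to the viewport, then casts player character 0 to BP_MyCharacter and stores the widget in that character's HUD variable.
; Releasing the F key calls AddHeart on the HUD with a false argument.
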(event EventBeginPlay
  (Utilities|FlowControl|Sequence
    (:then_0
      (bind _returnvalue (UserInterface|CreateWidget "/Game/BluePrints/GameHUD.GameHud_C" self))
      (bind _output_get (Variables|Default|SetGameHudRef _returnvalue))
      (UserInterface|Viewport|AddtoViewport _output_get 0)
      (bind _asbp_my_character (Utilities|Casting|CastToBP_MyCharacter (Game|GetPlayerCharacter 0)))
      (bind _output_get_2 (Variables|Default|SetMyCharacter _asbp_my_character))
      (Variables|/Game/BluePrints/BP_Mycharacter.BP_MyCharacter_C|SetHUD _output_get_2 (Variables|Default|GetGameHudRef)))))

(event Input|KeyboardEvents|F
  (params (Key :type Key%20Structure :default "None"))
  (:Released
    (Default|AddHeart (Variables|Default|GetGameHudRef) false)))

(fn ConstructionScript)